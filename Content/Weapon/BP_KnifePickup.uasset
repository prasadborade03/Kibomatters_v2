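; BP_KnifePickup is a knife pickup actor that shows a prompt widget while something overlaps its Overlap_e component.
; Interact prints a pickup message, calls DestroyKnife and returns the knife's static mesh to the caller.
; The destroy_knife event waits briefly, destroys the actor, then adds a Left_click widget to the first player's viewport, followed by a trailing delay with nothing after it.
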(event OnComponentBeginOverlap(overlap_e)
  (params (OverlappedComponent :type Primitive%20Component%20Object%20Reference) (OtherActor :type Actor%20Object%20Reference) (OtherComp :type Primitive%20Component%20Object%20Reference) (OtherBodyIndex :type Integer) (bFromSweep :type Boolean) (SweepResult :type Hit%20Result%20Structure%20%28by%20ref%29))
  (Rendering|SetVisibility (Variables|Default|GetWidget) true false))

(event OnComponentEndOverlap(overlap_e)
  (params (OverlappedComponent :type Primitive%20Component%20Object%20Reference) (OtherActor :type Actor%20Object%20Reference) (OtherComp :type Primitive%20Component%20Object%20Reference) (OtherBodyIndex :type Integer))
  (Rendering|SetVisibility (Variables|Default|GetWidget) false false))

(event Custom|destroy_knife
  (Utilities|FlowControl|Delay 0.2)
  (Actor|DestroyActor)
  (bind _returnvalue (UserInterface|CreateWidget "/Game/UI/MainMenu/left_click.left_click_C" (Game|GetPlayerController 0)))
  (UserInterface|Viewport|AddtoViewport _returnvalue 0)
  (Utilities|FlowControl|Delay 5.0))

(event EventBeginPlay)

(event Collision|EventActorBeginOverlap
  (params (OtherActor :type Actor%20Object%20Reference)))

(event EventTick
  (params (DeltaSeconds :type Float%20%28single-precision%29)))

(fn ConstructionScript)

(fn Interact
  (Development|PrintString "Picked Up")
  (CallFunction|DestroyKnife)
  (return (Variables|/Script/Engine.StaticMeshComponent|GetStaticMesh (Variables|Default|GetStaticMesh))))