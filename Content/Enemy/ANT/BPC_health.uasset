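; Health component in the ANT enemy folder that tracks Health and drives what happens when it runs out.
; Increases are clamped to a fixed range, decreases are not, and both broadcast UpdatedHealth.
; At zero or below, it broadcasts Dead, then switches on the player girl_bp's WhichLevel to open the main menu, show a TA widget, or open the end story level.
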(event EventBeginPlay)

(event EventTick
  (params (DeltaSeconds :type Float%20%28single-precision%29)))

(fn IncreaseHealth
  (params (Amount :type Float%20%28double-precision%29))
  (Variables|Default|Sethealth (Math|Float|Clamp(Float) (+ (Variables|Default|Gethealth) Amount) 0.0 1e+02))
  (Default|CallUpdatedHealth))

(fn DecreaseHealth
  (params (Damage :type Float%20%28double-precision%29))
  (bind _returnvalue (Game|GetPlayerController 0))
  (Variables|Default|Sethealth (- (Variables|Default|Gethealth) Damage))
  (Default|CallUpdatedHealth)
  (if (<= (Variables|Default|Gethealth) 0.0)
    (Default|CallDead)
    (bind _asgirl_bp (Utilities|Casting|CastTogirl_bp (Game|GetPlayerCharacter 0)))
    (switch int (Variables|/Game/ThirdPerson/Blueprints/girl_bp.girl_bp_C|Getwhich_level _asgirl_bp)
      (:0
        (Game|OpenLevel(byName) "MainMenuMap"))
      (:1
        (Game|OpenLevel(byName) "MainMenuMap"))
      (:2
        (bind _returnvalue_2 (UserInterface|CreateWidget "/Game/UI/MainMenu/level_3/TA1.TA1_C" _returnvalue))
        (UserInterface|Viewport|AddtoViewport _returnvalue_2 0))
      (:3
        (bind _returnvalue_3 (UserInterface|CreateWidget "/Game/UI/MainMenu/level_3/TA2.TA2_C" _returnvalue))
        (UserInterface|Viewport|AddtoViewport _returnvalue_3 0))
      (:4
        (bind _returnvalue_4 (UserInterface|CreateWidget "/Game/UI/MainMenu/level_3/TA3.TA3_C" _returnvalue))
        (UserInterface|Viewport|AddtoViewport _returnvalue_4 0))
      (:5
        (bind _returnvalue_5 (UserInterface|CreateWidget "/Game/UI/MainMenu/level_3/TA3.TA3_C" _returnvalue))
        (UserInterface|Viewport|AddtoViewport _returnvalue_5 0))
      (:6
        (Game|OpenLevel(byName) "end_story_level")))))