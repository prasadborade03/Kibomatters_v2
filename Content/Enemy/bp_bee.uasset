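; Bee enemy Blueprint that picks idle, chase or attack each Tick from its distance to the player.
; Idle computes a sine bob around the spawn point and chase a VInterpTo toward above the player, but both move the player controller, not the bee.
; Attack deals repeated damage through a DoOnce reset after a delay.
; AnyDamage is empty, and the health and destroy logic is disconnected.
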(event EventBeginPlay
  (Variables|Default|SetCachedPlayer (Game|GetPlayerCharacter 0))
  (Variables|Default|SetSpawnLocation (Transformation|GetActorLocation)))

(event EventTick
  (params (DeltaSeconds :type Float%20%28single-precision%29))
  (bind _returnvalue (Game|GetPlayerController 0))
  (bind _cachedplayer (Variables|Default|GetCachedPlayer))
  (bind _returnvalue_2 (Transformation|GetDistanceTo _cachedplayer 0))
  (if (< _returnvalue_2 1.5e+02)
    (Variables|Default|SetAIState 2)
    (elif (< _returnvalue_2 1.5e+03)
      (Variables|Default|SetAIState 1)
      (else
        (Variables|Default|SetAIState 0))))
  (switch int (Variables|Default|GetAIState)
    (:0
      (Transformation|SetActorLocation _returnvalue (+ (Variables|Default|GetSpawnLocation) (Math|Vector|MakeVector 0.0 0.0 (* 25.0 (Math|Trig|Sin(Radians) (Utilities|Time|GetGameTimeinSeconds))))) false false))
    (:1
      (Transformation|SetActorLocation _returnvalue (Math|Interpolation|VInterpTo "0, 0, 0" (+ (Transformation|GetActorLocation (Game|GetPlayerCharacter 0)) "0.000000,0.000000,50.000000") DeltaSeconds 5.0) false false))
    (:2
      (Utilities|FlowControl|DoOnce false :!label _label
        (:Completed
          (Game|Damage|ApplyDamage (Variables|Default|GetCachedPlayer) 1.0 0 0)
          (Utilities|FlowControl|Delay 1.2)
          (goto _label Reset))))))

(event Game|Damage|EventAnyDamage
  (params (Damage :type Float%20%28single-precision%29) (DamageType :type Damage%20Type%20Object%20Reference) (InstigatedBy :type Controller%20Object%20Reference) (DamageCauser :type Actor%20Object%20Reference)))

(fn ConstructionScript)