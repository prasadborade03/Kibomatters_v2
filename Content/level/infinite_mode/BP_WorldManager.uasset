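; World manager for infinite mode that streams HexChunkClass actors around the player.
; Tick converts the player's position to grid coordinates using 600-unit cells and calls UpdateChunks when they change, before storing the new coordinates.
; UpdateChunks thus centers on the previous chunk, spawning missing chunks in a 7x7 square into the SpawnedChunks map.
; It then destroys chunks beyond Manhattan distance 4, including that square's just-spawned corners.
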(event EventBeginPlay
  (bind (_q _r) (CallFunction|WorldtoChunk 0.0 0.0))
  (Variables|Default|SetPlayerRef (Game|Player|GetPlayerPawn 0))
  (Variables|Default|SetLastChunkQ _q)
  (Variables|Default|SetLastChunkR _r)
  (CallFunction|UpdateChunks))

(event Collision|EventActorBeginOverlap
  (params (OtherActor :type Actor%20Object%20Reference)))

(event EventTick
  (params (DeltaSeconds :type Float%20%28single-precision%29))
  (bind _playerref (Variables|Default|GetPlayerRef))
  (bind _returnvalue (Transformation|GetActorLocation _playerref))
  (bind (_q _r) (CallFunction|WorldtoChunk (.x _returnvalue) (.y _returnvalue)))
  (Utilities|IsValid _playerref
    (:Is%20Valid
      (if (or (!= (Variables|Default|GetLastChunkQ) _q) (!= _r (Variables|Default|GetLastChunkR)))
        (CallFunction|UpdateChunks)
        (Variables|Default|SetLastChunkQ _q)
        (Variables|Default|SetLastChunkR _r)))))

(fn ConstructionScript)

(fn UpdateChunks
  (for _index (range (- (Variables|Default|GetLastChunkQ) 3) (+ (Variables|Default|GetLastChunkQ) 3))
    (for _index_2 (range (- (Variables|Default|GetLastChunkR) 3) (+ (Variables|Default|GetLastChunkR) 3))
      (if (not (Utilities|Map|Contains (Variables|Default|GetSpawnedChunks) (Math|Vector2D|MakeVector2D (Math|Conversions|ToFloat(Integer) _index) (Math|Conversions|ToFloat(Integer) _index_2))))
        (bind _returnvalue (Game|SpawnActorfromClass (Variables|Default|GetHexChunkClass) (Math|Transform|MakeTransform (Math|Vector|MakeVector (Math|Conversions|ToFloat(Integer) (* _index (Variables|Default|GetChunkHeight))) (Math|Conversions|ToFloat(Integer) (* _index_2 (Variables|Default|GetChunkWidth))) 0.0) "0, 0, 0" "1.000000,1.000000,1.000000") "Undefined" "MultiplyWithRoot" 0 0))
        (Utilities|Map|Add (Variables|Default|GetSpawnedChunks) (Math|Vector2D|MakeVector2D (Math|Conversions|ToFloat(Integer) _index) (Math|Conversions|ToFloat(Integer) _index_2)) _returnvalue))))
  (bind _keys (Utilities|Map|Keys (Variables|Default|GetSpawnedChunks)))
  (for _array_element _keys
    (if (> (+ (Math|Float|Absolute(Float) (- (.x _array_element) (Variables|Default|GetLastChunkQ))) (Math|Float|Absolute(Float) (- (.y _array_element) (Variables|Default|GetLastChunkR)))) 4.0)
      (Actor|DestroyActor (.Value (Utilities|Map|Find (Variables|Default|GetSpawnedChunks) (Math|Vector2D|MakeVector2D (.x _array_element) (.y _array_element)))))
      (Utilities|Map|Remove (Variables|Default|GetSpawnedChunks) (Math|Vector2D|MakeVector2D (.x _array_element) (.y _array_element))))))

(fn WorldtoChunk
  (params (WorldX :type Float%20%28double-precision%29) (WorldY :type Float%20%28double-precision%29))
  (return (Math|Float|Floor (/ WorldX 6e+02)) (Math|Float|Floor (/ WorldY 6e+02))))